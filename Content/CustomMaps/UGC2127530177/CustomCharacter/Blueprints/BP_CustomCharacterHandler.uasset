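; Per-player custom character handler actor that removes itself when its player is gone or marked dead.
; The game logic actor sets a replicated setup flag, whose OnRep forces a net update and arms the local check.
; Once armed, the authority's Tick watches for an invalid owning PlayerState or a "dead" tag on itself, its owner or the PlayerState.
; Either condition sets its lifespan once, scheduling destruction.
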(event `self.ReceiveTick`
  (params (DeltaSeconds :type "Float (single-precision)"))
  ;[1 1 1] Handle killing self on player tag 'dead'
  (`/Engine/EditorBlueprintResources/ActorMacros.Switch Has Authority`
    (:`Authority`
      (if (`self.PerActor_LocalSetUp`)
        (`|ExecutionSequence`
          (:`then_0`
            ;[1 1 1] Check if player state is valid. False if player is not connected?
            (if (not (`KismetSystemLibrary.IsValid` (`self.OwningPlayerState`)))
              ;[1 1 1] Kill self
              (`/Engine/EditorBlueprintResources/StandardMacros.DoOnce` false :!label _label
                (:`Completed`
                  (`self.SetLifeSpan` (`self.Lifespan`))))))
          (:`then_1`
            ;[1 1 1] Check actor tags for 'dead' tag
            (if (or (`self.ActorHasTag` (`self.GetOwner`) "dead") (`self.ActorHasTag` self "dead") (`self.ActorHasTag` (`self.OwningPlayerState`) "dead"))
              (goto _label))))))))

(fn `OnRep_PerActorSetup`
  ;[1 1 1] Once PerActorLocalSetUp variable is set true, this actor can be killed by the game logic. This variable is set by the game logic actor
  (`/Engine/EditorBlueprintResources/ActorMacros.Switch Has Authority`
    (:`Authority`
      _)
    (:`Remote`
      _))
  (if (`self.PerActorSetup`)
    (`self.ForceNetUpdate`)
    (set `self.PerActor_LocalSetUp` true)))

(fn `UserConstructionScript`)