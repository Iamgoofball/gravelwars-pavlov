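; Server-side Pavlov custom game mode that runs timed rounds and a timed match while replacing player meshes with team-based custom characters.
; On spawn it creates a BP_CustomCharacter and team handler linked to the Pavlov skeleton, scaled by root-to-head height.
; "Dead" tags, a polling timer and join-time re-setup keep characters in sync.
; Round changes clean up characters, respawn players and notify BPI_MatchRounds actors.
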(event `self.OnCustomGameModeInit`
  ;[1 1 1] Init GameMode Properties when server starts
  (`self.SetGameModeProperties` (make `PavlovGameModeProperties` false true false 99999 10000 0 false true 5.0 false false 30 10 true true 45)))

(event `self.OnPlayerSpawned`
  (params (PlayerStatus :type "PavlovPlayerStatus Structure (by ref)"))
  (bind (_playerstate _controller _pawn) (break `PavlovPlayerStatus` PlayerStatus))
  (bind _array (`|MakeArray` "None" :!type "Name"))
  ;[1 0.3263 0.3123 1 170] Custom Character Logic
  ;;[1 1 1] On Player Spawn
  (`/Engine/EditorBlueprintResources/ActorMacros.Switch Has Authority`
    (:`Authority`
      (`/CustomMapTools/Blueprints/BPFL_PavlovTemplate.ManageTags` _playerstate false "dead")
      (set `Actor.Tags` _array _controller)
      (set `Actor.Tags` _array _pawn)
      (`self.SetPlayerBuyingEnabled` _playerstate 120.0 3000.0)
      (bind (_sk_mesh _success) (`self.GetPavSkel` _pawn))
      (if _success
        (`|ExecutionSequence`
          (:`then_0`
            (`self.SpawnCustomCharacter` PlayerStatus 4.0))
          (:`then_1`
            (bind _customcharacter (`self.GetOwnedCustomCharacter` _pawn))
            (`self.Scale to Pavlov Skeleton` _customcharacter _sk_mesh)))))))

(event `self.OnPlayerKilled`
  (params (PlayerStatus :type "PavlovPlayerStatus Structure (by ref)") (Killer :type "PlayerState Object Reference") (bHeadshot :type Boolean) (KilledByItem :type Name))
  (bind (_playerstate _controller _pawn) (break `PavlovPlayerStatus` PlayerStatus))
  (bind _array (`|MakeArray` "dead" :!type "Name"))
  ;[1 0.3263 0.3123 1 170] Custom Character Logic
  ;;[1 1 1] On Player Killed
  (`/Engine/EditorBlueprintResources/ActorMacros.Switch Has Authority`
    (:`Authority`
      (`/CustomMapTools/Blueprints/BPFL_PavlovTemplate.ManageTags` _playerstate true "dead")
      (set `Actor.Tags` _array _controller)
      (set `Actor.Tags` _array _pawn))))

(event `SpawnCustomCharacter`
  (params (PlayerStatus :type "PavlovPlayerStatus Structure") (CharacterRagdollTime :type "Float (double-precision)"))
  (bind (_playerstate _controller _pawn _steamid _cash _score _teamid) (break `PavlovPlayerStatus` PlayerStatus))
  (bind _returnvalue (`self.GetTransform` _pawn))
  ;[1 0.3263 0.3123 1 170] Custom Character Logic
  ;;[1 1 1] Spawn character mesh to replace pavlov mesh
  (`/Engine/EditorBlueprintResources/ActorMacros.Switch Has Authority`
    (:`Authority`
      (bind _returnvalue_2 (`|SpawnActorFromClass` "/Game/CustomMaps/UGC2127530177/CustomCharacter/Blueprints/BP_CustomCharacter.BP_CustomCharacter_C" _returnvalue "AlwaysSpawn" "OverrideRootScale" _pawn null))
      (set `Actor.NetPriority` 99.0 _returnvalue_2)
      (`self.SetReplicates` _returnvalue_2 true)
      (`self.SetReplicates` (stale _returnvalue_3) true)
      (bind _returnvalue_3 (`|SpawnActorFromClass` (`|GetArrayItem` (`self.CharacterSpawnArray`) _teamid) _returnvalue "AlwaysSpawn" "OverrideRootScale" _pawn null))
      (set `Actor.bNetUseOwnerRelevancy` true _returnvalue_3)
      (`self.SetReplicates` _returnvalue_3 true)
      (`ActorComponent.SetIsReplicated` (`Character.Mesh` _returnvalue_3) true)
      (`ActorComponent.SetIsReplicated` (`Character.CapsuleComponent` _returnvalue_3) true)
      (bind _sk_mesh (`self.GetPavSkel` _pawn))
      ;;;[1 1 1] BP_CustomCharacterHandler Parameters
      (set `/Game/CustomMaps/UGC2127530177/CustomCharacter/Blueprints/BP_CustomCharacterHandler.Lifespan` CharacterRagdollTime _returnvalue_3)
      (set `/Game/CustomMaps/UGC2127530177/CustomCharacter/Blueprints/BP_CustomCharacterHandler.OwningPlayerState` _playerstate _returnvalue_3)
      ;;;[1 1 1] BP_CustomCharater Parameters
      (set `/Game/CustomMaps/UGC2127530177/CustomCharacter/Blueprints/BP_CustomCharacter.OwningPlayerState` _playerstate _returnvalue_2)
      (set `/Game/CustomMaps/UGC2127530177/CustomCharacter/Blueprints/BP_CustomCharacter.Lifespan` CharacterRagdollTime _returnvalue_2)
      (set `/Game/CustomMaps/UGC2127530177/CustomCharacter/Blueprints/BP_CustomCharacter.Character` _returnvalue_3 _returnvalue_2) ; Character Object
      (set `/Game/CustomMaps/UGC2127530177/CustomCharacter/Blueprints/BP_CustomCharacter.ParentPawn` _pawn _returnvalue_2)
      (set `/Game/CustomMaps/UGC2127530177/CustomCharacter/Blueprints/BP_CustomCharacter.ParentSkelToCopy` _sk_mesh _returnvalue_2) ; Parent Pavlov Skel Mesh
      (`KismetSystemLibrary.Delay` 0.2)
      (set `/Game/CustomMaps/UGC2127530177/CustomCharacter/Blueprints/BP_CustomCharacter.AllComponentsSet` true _returnvalue_2)
      (set `/Game/CustomMaps/UGC2127530177/CustomCharacter/Blueprints/BP_CustomCharacterHandler.PerActorSetup` true _returnvalue_3))))

(event `self.ReceiveBeginPlay`
  ;[1 1 1] Time till game starts
  (`/Engine/EditorBlueprintResources/ActorMacros.Switch Has Authority`
    (:`Authority`
      (`KismetSystemLibrary.Delay` 5.0)
      (`self.SetRoundState` "StandBy")
      (`KismetSystemLibrary.Delay` 3.0)
      (`self.SetRoundState` "Started")
      (`self.Match Timer`)
      ;;[1 0.4156 0.4156] Set current player array and start Character State Update Timer
      (bind _players (`self.GetPlayers`))
      (set `self.CurrentPlayerArray` _players)
      (`self.CharacterStateUpdateTimer`))))

(event `self.OnPlayerJoinedServer`
  (params (PlayerStatus :type "PavlovPlayerStatus Structure (by ref)"))
  (bind (_playerstate _controller _pawn) (break `PavlovPlayerStatus` PlayerStatus))
  (bind _array (`|MakeArray` "None" :!type "Name"))
  ;[1 1 1] OnPlayerJoinedServer
  (`KismetArrayLibrary.Array_AddUnique` (`self.ConnectedPlayers`) _playerstate)
  (set `Actor.Tags` _array _controller)
  (set `Actor.Tags` _array _pawn)
  ;;[1 0.2643 0.2105] Custom Character Logic
  (`self.SetupExistingCharactersOnJoin`))

(event `Scale to Pavlov Skeleton`
  (params (Character :type "/Game/CustomMaps/UGC2127530177/CustomCharacter/Blueprints/BP_CustomCharacterHandler Object Reference") (PavSkel :type "SkeletalMeshComponent Object Reference"))
  ;[1 0.3263 0.3123 1 170] Custom Character Logic
  ;;[1 1 1] Scaling the model to match pavlov model
  (`/Engine/EditorBlueprintResources/ActorMacros.Switch Has Authority`
    (:`Authority`
      (bind _distancefromheadtoroot (`self.GetHeightOfSkel` (`Character.Mesh` Character))) ; CustomCharacter
      (bind _distancefromheadtoroot_2 (`self.GetHeightOfSkel` PavSkel)) ; PavPawn
      (bind _returnvalue (* (/ _distancefromheadtoroot_2 _distancefromheadtoroot) 1.05))
      (`SceneComponent.SetWorldScale3D` (`Actor.RootComponent` Character) (`KismetMathLibrary.MakeVector` _returnvalue _returnvalue _returnvalue)))))

(event `Play Sound FX 2D`
  (params (Sound :type "SoundBase Object Reference"))
  ;[1 1 1] Example of replicated 2d sound effect (make sure to call from server)
  (`GameplayStatics.PlaySound2D` Sound 1.0 1.0 0.0 null null))

(event `SetupExistingCharactersOnJoin`
  ;[1 0.3263 0.3123 1 170] Custom Character Logic
  ;;[1 1 1] SetupExistingCharacters
  (`/Engine/EditorBlueprintResources/ActorMacros.Switch Has Authority`
    (:`Authority`
      (`|ExecutionSequence`
        (:`then_0`
          ;;;[1 1 1] 1. For all custom character actors, if AllComponentsSet is true, call it again.
          (bind _outactors (`GameplayStatics.GetAllActorsOfClass` "/Game/CustomMaps/UGC2127530177/CustomCharacter/Blueprints/BP_CustomCharacter.BP_CustomCharacter_C"))
          (for _array_element _outactors
            (if (`/Game/CustomMaps/UGC2127530177/CustomCharacter/Blueprints/BP_CustomCharacter.AllComponentsSet` _array_element)
              (if (not (`/Game/CustomMaps/UGC2127530177/CustomCharacter/Blueprints/BP_CustomCharacter.IsKilled` _array_element))
                (set `/Game/CustomMaps/UGC2127530177/CustomCharacter/Blueprints/BP_CustomCharacter.AllComponentsSet` true _array_element))
              (else
                ;;;[1 1 1] If AllComponentsSet is false, and the pawn is not a pavlov pawn, then set IsKilled true to kill the character.
                (bind _aspawn (cast `Pawn` (`self.GetOwner` _array_element))
                  (:`then`
                    (if (`/CustomMapTools/Blueprints/BPFL_PavlovTemplate.IsPavPawn?` _aspawn)
                      (bind (_playerstatus _bsucceeded) (`PavlovProxyStatics.GetPavlovPlayerStatusByPawn` _aspawn))
                      (if _bsucceeded
                        ;;;[1 1 1] If it is a Pavlov pawn, then pass all parameters back to the CustomCharacter and Handler and call the replicated setup variables
                        (for _array_element_2 (`self.GetAllChildActors` _aspawn true)
                          (bind _asbp_custom_character_handler (cast `/Game/CustomMaps/UGC2127530177/CustomCharacter/Blueprints/BP_CustomCharacterHandler` _array_element_2))
                          (set `/Game/CustomMaps/UGC2127530177/CustomCharacter/Blueprints/BP_CustomCharacterHandler.Lifespan` (`self.GlobalLifespan`) _asbp_custom_character_handler)
                          (bind (_playerstate _controller _pawn) (break `PavlovPlayerStatus` _playerstatus))
                          (set `/Game/CustomMaps/UGC2127530177/CustomCharacter/Blueprints/BP_CustomCharacterHandler.OwningPlayerState` _playerstate _asbp_custom_character_handler)
                          (set `/Game/CustomMaps/UGC2127530177/CustomCharacter/Blueprints/BP_CustomCharacter.Character` _asbp_custom_character_handler _array_element) ; Character Object
                          (set `/Game/CustomMaps/UGC2127530177/CustomCharacter/Blueprints/BP_CustomCharacterHandler.PerActorSetup` true _asbp_custom_character_handler))
                        (set `/Game/CustomMaps/UGC2127530177/CustomCharacter/Blueprints/BP_CustomCharacter.OwningPlayerState` _playerstate _array_element)
                        (set `/Game/CustomMaps/UGC2127530177/CustomCharacter/Blueprints/BP_CustomCharacter.Lifespan` (`self.GlobalLifespan`) _array_element)
                        (bind _output_get (set `/Game/CustomMaps/UGC2127530177/CustomCharacter/Blueprints/BP_CustomCharacter.ParentPawn` _pawn _array_element))
                        (bind _sk_mesh (`self.GetPavSkel` _output_get))
                        (set `/Game/CustomMaps/UGC2127530177/CustomCharacter/Blueprints/BP_CustomCharacter.ParentSkelToCopy` _sk_mesh _array_element) ; Parent Pavlov Skel Mesh
                        (set `/Game/CustomMaps/UGC2127530177/CustomCharacter/Blueprints/BP_CustomCharacter.AllComponentsSet` true _array_element)
                        (else
                          (set `/Game/CustomMaps/UGC2127530177/CustomCharacter/Blueprints/BP_CustomCharacter.IsKilled` true _array_element :!label _label)))
                      (else
                        (goto _label))))
                  (:`CastFailed`
                    (goto _label)))))))
        (:`then_1`
          ;;;[1 1 1] 2. For all actors Custom Character Handler, if their player state is valid, call PerActorSetup
          (bind _outactors_2 (`GameplayStatics.GetAllActorsOfClass` "/Game/CustomMaps/UGC2127530177/CustomCharacter/Blueprints/BP_CustomCharacterHandler.BP_CustomCharacterHandler_C"))
          (for _array_element_3 _outactors_2
            (if (`KismetSystemLibrary.IsValid` (`/Game/CustomMaps/UGC2127530177/CustomCharacter/Blueprints/BP_CustomCharacterHandler.OwningPlayerState` _array_element_3))
              (set `/Game/CustomMaps/UGC2127530177/CustomCharacter/Blueprints/BP_CustomCharacterHandler.PerActorSetup` true _array_element_3))))))))

(event `self.OnPlayerLeftServer`
  (params (PlayerStatus :type "PavlovPlayerStatus Structure (by ref)"))
  (bind (_playerstate _controller _pawn) (break `PavlovPlayerStatus` PlayerStatus))
  (bind _array (`|MakeArray` "dead" :!type "Name"))
  ;[1 1 1] OnPlayerLeftServer
  (`KismetArrayLibrary.Array_RemoveItem` (`self.ConnectedPlayers`) _playerstate)
  (`/CustomMapTools/Blueprints/BPFL_PavlovTemplate.ManageTags` _playerstate true "dead")
  (set `Actor.Tags` _array _controller)
  (set `Actor.Tags` _array _pawn))

(event `Play Sound FX At Location`
  (params (Sound :type "SoundBase Object Reference") (Location :type "Vector Structure"))
  ;[1 1 1] Example of replicated sound that plays at a location (use cues for attenuation, call from server)
  (`GameplayStatics.PlaySoundAtLocation` Sound Location (struct) 1.0 1.0 0.0 null null null))

(event `self.OnRoundBegin`
  ;[1 1 1] OnRoundBegin
  (`KismetSystemLibrary.Delay` 4.0)
  (bind _players (`self.GetPlayers`))
  (for _array_element _players
    (`KismetSystemLibrary.Delay` 0.1)
    (bind (_playerstatus _bsucceeded) (`PavlovProxyStatics.GetPavlovPlayerStatus` _array_element))
    (if _bsucceeded
      (if (`.bDead` (break `PavlovPlayerStatus` _playerstatus))
        (`self.RespawnPlayer` _playerstatus))
      (`self.SetPlayerBuyingEnabled` _array_element 45.0 2000.0)))
  (`self.SetRoundState` "StandBy")
  (`self.SetMovementDisabled` true)
  (`KismetSystemLibrary.Delay` 1.0)
  (`self.SetMovementDisabled` false)
  (`self.SetRoundState` "Started"))

(event `self.OnRoundEnd`
  ;[1 1 1] OnRoundEnd
  (`/Engine/EditorBlueprintResources/StandardMacros.DoOnce` false :!label _label_2
    (:`Completed`
      (`self.CleanUpCustomCharacters`)
      (for _array_element (`GameStateBase.PlayerArray` (`GameplayStatics.GetGameState`))
        (bind (_playerstatus _bsucceeded) (`PavlovProxyStatics.GetPavlovPlayerStatus` _array_element))
        (if _bsucceeded
          (bind (_playerstate _controller _pawn _steamid _cash _score _teamid _health _armour _bhelmet _bdead) (break `PavlovPlayerStatus` _playerstatus))
          (if (not _bdead)
            (`/CustomMapTools/Blueprints/BPFL_PavlovTemplate.ManageTags` _playerstate true "dead")
            (`GameplayStatics.ApplyDamage` _pawn 500.0))))
      (`self.PostRoundCleanUp`)
      (`KismetSystemLibrary.Delay` 1.0)
      (`self.SetRoundState` "Starting")
      (goto _label_2 :!via `Reset`))))

(event `CleanUpCustomCharacters`
  ;[1 0.3263 0.3123 1 170] Custom Character Logic
  ;;[1 1 1] Clean Up All Custom Characters on Round Begin
  (`/Engine/EditorBlueprintResources/ActorMacros.Switch Has Authority`
    (:`Authority`
      (bind _outactors (`GameplayStatics.GetAllActorsOfClass` "/Game/CustomMaps/UGC2127530177/CustomCharacter/Blueprints/BP_CustomCharacter.BP_CustomCharacter_C"))
      (for _array_element _outactors
        (set `Actor.Tags` (`|MakeArray` "dead" :!type "Name") _array_element))
      (`KismetSystemLibrary.Delay` 1.0)
      (bind _outactors_2 (`GameplayStatics.GetAllActorsOfClass` "/Game/CustomMaps/UGC2127530177/CustomCharacter/Blueprints/BP_CustomCharacterHandler.BP_CustomCharacterHandler_C"))
      (for _array_element_2 _outactors_2
        (set `Actor.Tags` (`|MakeArray` "dead" :!type "Name") _array_element_2)))))

(event `CharacterStateUpdateTimer`
  ;[1 0.3263 0.3123 1 170] Custom Character Logic
  ;;[1 1 1] Character State Update Timer: checks if each connected player is dead, or if they no longer are in the game to kill their spawned custom characters
  (`/Engine/EditorBlueprintResources/ActorMacros.Switch Has Authority`
    (:`Authority`
      (`KismetSystemLibrary.K2_SetTimerDelegate` (delegate `UpdateCharacterStates`) 1.0 true))))

(event `UpdateCharacterStates`
  ;[1 0.3263 0.3123 1 170] Custom Character Logic
  ;;[1 1 1] Character State Update Timer: checks if each connected player is dead, or if they no longer are in the game to kill their spawned custom characters
  (`/Engine/EditorBlueprintResources/StandardMacros.DoOnce` false :!label _label_3
    (:`Completed`
      ;;;[1 1 1] Get all connected players and compare the array to the array currently stored in the variable from the last time this function was called. For each player in the old array, check if the new array contains the old element
      (bind _players (`self.GetPlayers`))
      (for _array_element (`self.CurrentPlayerArray`)
        (if (`KismetArrayLibrary.Array_Contains` _players _array_element)
          ;;;[1 1 1] If player is still in the game, check if they are dead. If so, kill their character  by setting 'dead' tag on player state
          (bind (_playerstatus _bsucceeded) (`PavlovProxyStatics.GetPavlovPlayerStatus` _array_element))
          (if _bsucceeded
            (bind (_playerstate _controller _pawn _steamid _cash _score _teamid _health _armour _bhelmet _bdead) (break `PavlovPlayerStatus` _playerstatus))
            (if (or (not (`/CustomMapTools/Blueprints/BPFL_PavlovTemplate.IsPavPawn?` _pawn)) _bdead)
              (`/CustomMapTools/Blueprints/BPFL_PavlovTemplate.ManageTags` _array_element true "dead" :!label _label_4))
            (else
              (goto _label_4)))
          (else
            ;;;[1 1 1] If player is not in the new array, check if their pawn is dead or if their player status is gettable. If dead or status not gettable, set 'dead'.
            (bind (_playerstatus_2 _bsucceeded_2) (`PavlovProxyStatics.GetPavlovPlayerStatus` _array_element))
            (if _bsucceeded_2
              (bind (_playerstate_2 _controller_2 _pawn_2 _steamid_2 _cash_2 _score_2 _teamid_2 _health_2 _armour_2 _bhelmet_2 _bdead_2) (break `PavlovPlayerStatus` _playerstatus_2))
              (if (`/CustomMapTools/Blueprints/BPFL_PavlovTemplate.IsPavPawn?` _pawn_2)
                (if _bdead_2
                  (goto _label_4))
                (else
                  (goto _label_4)))
              (else
                (goto _label_4))))))
      ;;;[1 1 1] Store new array for next call
      (`KismetSystemLibrary.Delay` 1.0)
      (`self.SetupExistingCharactersOnJoin`)
      (set `self.CurrentPlayerArray` _players)
      (goto _label_3 :!via `Reset`))))

(event `Match Timer`
  ;[1 1 1] Time till match ends
  ; End match can be called due to specific requirements being met vs having it on a timer.
  (`KismetSystemLibrary.K2_SetTimerDelegate` (delegate `End Match`) 600.0))

(event `End Match`
  ;[1 1 1] Time till match ends
  ; End match can be called due to specific requirements being met vs having it on a timer.
  (`/Engine/EditorBlueprintResources/StandardMacros.DoOnce` false
    (:`Completed`
      (bind _asgame_mode (cast `GameMode` (`GameplayStatics.GetGameMode`)))
      (`GameMode.EndMatch` _asgame_mode))))

(event `self.OnRoundStateChanged`
  (params (OldState :type "EPavlovRoundState Enum" :default "Starting") (NewState :type "EPavlovRoundState Enum" :default "Starting"))
  ;[1 1 1] Updates all blueprints with BPI_MatchRounds implemented,
  ;  can be used to reset actors to initial state (Ill cover this in the video)
  (`self.RoundInterfaceCall` NewState)
  (`KismetSystemLibrary.PrintString` (`KismetStringLibrary.Concat_StrStr` (`|GetEnumeratorNameAsString` OldState) "||" (`|GetEnumeratorNameAsString` NewState))))

(fn `GetConnectedPawns`
  (returns (AlivePawns :type "Array of Pawn Object Reference") (AliveCount :type Integer) (GhostPawns :type "Array of Pawn Object Reference") (GhostCount :type Integer))
  (locals (L_AliveCount :type Integer :default 0) (L_AlivePawns :type "Array of Pawn Object Reference") (L_GhostCount :type Integer) (L_GhostPawns :type "Array of Pawn Object Reference"))
  (for _array_element (`self.ConnectedPlayers`)
    (bind (_playerstatus _bsucceeded) (`PavlovProxyStatics.GetPavlovPlayerStatus` _array_element))
    (if _bsucceeded
      (bind (_playerstate _controller _pawn) (break `PavlovPlayerStatus` _playerstatus))
      (if (`/CustomMapTools/Blueprints/BPFL_PavlovTemplate.IsPavPawn?` _pawn)
        (`/Engine/EditorBlueprintResources/StandardMacros.IncrementInt` (`local.L_AliveCount`)
          (:`  `
            (`KismetArrayLibrary.Array_AddUnique` (`local.L_AlivePawns`) _pawn)))
        (else
          (`/Engine/EditorBlueprintResources/StandardMacros.IncrementInt` (`local.L_GhostCount`)
            (:`  `
              (`KismetArrayLibrary.Array_AddUnique` (`local.L_GhostPawns`) _pawn)))))))
  (return (`local.L_AlivePawns`) (`local.L_AliveCount`) (`local.L_GhostPawns`) (`local.L_GhostCount`)))

(fn `GetHeightOfSkel`
  (params (Mesh :type "SkeletalMeshComponent Object Reference"))
  (returns (DistanceFromHeadToRoot :type "Float (double-precision)"))
  (locals (RootNode :type "Actor Object Reference") (HeadNode :type "Actor Object Reference"))
  (return (`KismetAnimationLibrary.K2_DistanceBetweenTwoSocketsAndMapRange` Mesh "root" "RTS_World" "head" "RTS_World")))

(fn `GetOwnedCustomCharacter`
  (params (Pawn :type "Pawn Object Reference"))
  (returns (CustomCharacter :type "/Game/CustomMaps/UGC2127530177/CustomCharacter/Blueprints/BP_CustomCharacterHandler Object Reference") (Success :type Boolean))
  (for _array_element (`self.GetAllChildActors` Pawn true)
    (bind _asbp_custom_character_handler (cast `/Game/CustomMaps/UGC2127530177/CustomCharacter/Blueprints/BP_CustomCharacterHandler` _array_element))
    (return _asbp_custom_character_handler true))
  (return null false))

(fn `GetPavSkel`
  (params (PavPawn :type "Pawn Object Reference"))
  (returns (`SK Mesh` :type "SkeletalMeshComponent Object Reference") (Success :type Boolean))
  (if (`/CustomMapTools/Blueprints/BPFL_PavlovTemplate.IsPavPawn?` PavPawn)
    (bind _ascharacter (cast `Character` (`local.PavPawn`))
      (:`then`
        (return (`|GetArrayItem` (`self.K2_GetComponentsByClass` _ascharacter "/Script/Engine.SkeletalMeshComponent") 1) true))
      (:`CastFailed`
        (return null false)))))

(fn `GetPlayers`
  (returns (Players :type "Array of PlayerState Object Reference"))
  (bind _asgame_state (cast `GameState` (`GameplayStatics.GetGameState`)))
  (return (`GameStateBase.PlayerArray` _asgame_state)))

(fn `OnAssignTeam`
  (params (Status :type "PavlovPlayerStatus Structure (by ref)"))
  (returns (TeamId :type Integer))
  (if (> 0 0)
    (return 0)
    (else
      (return 1))))

(fn `RespawnPlayer`
  (params (PlayerStatus :type "PavlovPlayerStatus Structure (by ref)") (`As Ghost` :type Boolean) (`Spawn At Transform?` :type Boolean) (Transform :type "Transform Structure"))
  (bind (_playerstate _controller) (break `PavlovPlayerStatus` PlayerStatus))
  (if (`local.Spawn At Transform?`)
    (`self.Spawn` _controller (`local.Transform`) (`local.As Ghost`))
    (else
      (bind _transform (`self.GetSpawnTransform` _controller))
      (`self.Spawn` _controller _transform (`local.As Ghost`))))
  (return))

(fn `RoundInterfaceCall`
  (params (`Round State` :type "EPavlovRoundState Enum" :default "Starting"))
  (locals (L_InterfaceActors :type "Array of Actor Object Reference"))
  (bind _l_interfaceactors (`local.L_InterfaceActors`))
  (bind _outactors (`GameplayStatics.GetAllActorsWithInterface` "/CustomMapTools/Blueprints/BPI_MatchRounds.BPI_MatchRounds_C"))
  (set `local.L_InterfaceActors` _outactors)
  (switch `EPavlovRoundState` (`local.Round State`)
    (:`Starting`
      (message `/CustomMapTools/Blueprints/BPI_MatchRounds.RoundStarting` _l_interfaceactors))
    (:`StandBy`
      (message `/CustomMapTools/Blueprints/BPI_MatchRounds.RoundStandBy` _l_interfaceactors))
    (:`Started`
      (message `/CustomMapTools/Blueprints/BPI_MatchRounds.RoundStarted` _l_interfaceactors))
    (:`Ended`
      (message `/CustomMapTools/Blueprints/BPI_MatchRounds.RoundEnded` _l_interfaceactors)))
  (return))

(fn `UserConstructionScript`)