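; Replicated custom character manager that replaces a Pavlov player's visible body with a custom model.
; When AllComponentsSet replicates, it attaches Character to the pawn's skeleton, passes that mesh to the AnimInstance for pose copying, and hides the model from its owner.
; The original meshes are hidden but forced to keep full-rate animation.
; Server Tick sets IsKilled on an invalid PlayerState or "dead" tag, starting the actor's lifespan countdown.
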(event `self.ReceiveTick`
  (params (DeltaSeconds :type "Float (single-precision)"))
  ;[1 1 1] Handle killing character when pawn dies
  (`/Engine/EditorBlueprintResources/ActorMacros.Switch Has Authority`
    (:`Authority`
      (if (and (`self.AllComponentsSet`) (`self.LocalSetUp`))
        (`|ExecutionSequence`
          (:`then_0`
            ;[1 1 1] Check Player State is valid
            (if (not (`KismetSystemLibrary.IsValid` (`self.OwningPlayerState`)))
              (set `self.IsKilled` true)))
          (:`then_1`
            ;[1 1 1] Check if self or player state has dead tag
            (if (or (`self.ActorHasTag` (`self.GetOwner`) "dead") (`self.ActorHasTag` self "dead") (`self.ActorHasTag` (`self.OwningPlayerState`) "dead") (`self.ActorHasTag` (`self.Character`) "dead") (`self.ActorHasTag` (`self.PlayerController`) "dead"))
              (set `Actor.Tags` (`|MakeArray` "dead" :!type "Name") (`self.Character`))
              (set `self.IsKilled` true))))))))

(fn `GetHeightOfSkel`
  (params (SkelMesh :type "SkeletalMeshComponent Object Reference"))
  (returns (DistanceFromHeadToRoot :type "Float (double-precision)"))
  (return (`KismetAnimationLibrary.K2_DistanceBetweenTwoSocketsAndMapRange` SkelMesh "root" "RTS_World" "head" "RTS_World")))

(fn `OnRep_AllComponentsSet`
  (bind _character (`self.Character`))
  (bind _parentskeltocopy (`self.ParentSkelToCopy`))
  (bind _parentskeltocopy_2 (`self.ParentSkelToCopy`))
  (bind _parentskeltocopy_3 (`self.ParentSkelToCopy`))
  (bind _returnvalue_location (`KismetMathLibrary.BreakTransform` (`SceneComponent.GetSocketTransform` _parentskeltocopy "root" "RTS_World")))
  (bind _mesh (`Character.Mesh` _character))
  (bind _output (`|GetArrayItem` (`self.K2_GetComponentsByClass` (`self.ParentPawn`) "/Script/Engine.SkinnedMeshComponent") 4))
  ;[1 1 1] Comment
  (`/Engine/EditorBlueprintResources/ActorMacros.Switch Has Authority` ; This must run on client and server for client to see\nplayer mesh being copied
    (:`Authority`
      _)
    (:`Remote`
      _))
  (if (`self.AllComponentsSet`)
    ;[1 1 1] Set up custom mesh
    (`self.SetReplicates` _character true)
    (`ActorComponent.SetIsReplicated` (`Character.CapsuleComponent` _character) true)
    (`ActorComponent.SetIsReplicated` _mesh true)
    (`self.K2_AttachToComponent` _character _parentskeltocopy_2 "root" "SnapToTarget" "SnapToTarget" "SnapToTarget" true)
    (`SceneComponent.K2_SetWorldRotation` _mesh (`KismetMathLibrary.Conv_VectorToRotator` (`SceneComponent.GetForwardVector` _parentskeltocopy_2)) false false) ; Rotate spawned player model to match parent's
    (`PrimitiveComponent.SetOwnerNoSee` _mesh true) ; Hides custom model from pawn owner\nIf disabled, player can see their body
    (message `/Game/CustomMaps/UGC2127530177/CustomCharacter/Blueprints/BPI_CustomCharacterInterface.SetPavlovSkelMeshToCopy` (`SkeletalMeshComponent.GetAnimInstance` _mesh) _parentskeltocopy)
    (`SceneComponent.K2_SetWorldLocation` (`Character.Mesh` (`self.Character`)) _returnvalue_location false false) ; This moves the spawned model's root to match parent's.\nWithout this, the model is in the floor
    ;[1 1 1] Set pavlov player model invisible.
    (`SceneComponent.SetVisibility` _parentskeltocopy_3 false false)
    (`SceneComponent.SetVisibility` _output false false)
    ;[1 1 1] This disables update rate opitimizations that would cause the pavlov player model to be play at half frame rate because it is invisible.
    (set `SkinnedMeshComponent.bEnableUpdateRateOptimizations` false _parentskeltocopy_3)
    (set `SkinnedMeshComponent.VisibilityBasedAnimTickOption` "AlwaysTickPoseAndRefreshBones" _parentskeltocopy_3)
    (set `SkinnedMeshComponent.bEnableUpdateRateOptimizations` false _output)
    (set `SkinnedMeshComponent.VisibilityBasedAnimTickOption` "AlwaysTickPoseAndRefreshBones" _output)
    (set `self.LocalSetUp` true) ; Per-client, tracks if character is set up locally to copy animations
  ))

(fn `OnRep_IsKilled`
  ;[1 1 1] Handle killing self on server
  (`/Engine/EditorBlueprintResources/ActorMacros.Switch Has Authority`
    (:`Authority`
      (`/Engine/EditorBlueprintResources/StandardMacros.DoOnce` false
        (:`Completed`
          (`self.SetLifeSpan` (`self.Lifespan`)))))))

(fn `UserConstructionScript`)