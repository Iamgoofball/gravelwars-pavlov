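; Payload cart for a TF2-style Pavlov mode that players push along a chain of spline track segments.
; The CartMover timeline counts living players in PlayerSensor, scales speed up to three pushers, and checks teams to block pushing.
; Unpushed carts roll back immediately on hill tracks, otherwise after a delay.
; GameLaws receives checkpoint alerts, and segment ends trigger captures, advance to the next track or end the round.
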(event `ResetCartToFirstTrack`
  (bind _starting_track (`self.Starting Track`))
  (bind _trackspline (`/Game/CustomMaps/UGC1662809422/BluePrints/PL/Track_Node.TrackSpline` _starting_track))
  (bind _returnvalue (`KismetMathLibrary.Lerp` 0.0 (`SplineComponent.GetSplineLength` _trackspline) (`self.Alpha`)))
  (set `self.resetting` true)
  (set `self.Track` _starting_track)
  (`self.MoveCartMulticast`)
  (`TimelineComponent.SetNewTime` (`self.cartMover`) 0.0)
  (set `self.CartStartOffset` 0.0)
  (`self.K2_SetActorLocationAndRotation` (`SplineComponent.GetLocationAtDistanceAlongSpline` _trackspline _returnvalue "World") (`SplineComponent.GetRotationAtDistanceAlongSpline` _trackspline _returnvalue "World") false true)
  (set `self.alerted` false)
  (set `self.resetting` false))

(event `self.PlayerSensor.OnComponentBeginOverlap`
  (params (OverlappedComponent :type "PrimitiveComponent Object Reference") (OtherActor :type "Actor Object Reference") (OtherComp :type "PrimitiveComponent Object Reference") (OtherBodyIndex :type Integer) (bFromSweep :type Boolean) (SweepResult :type "HitResult Structure (by ref)"))
  (bind _track (`self.Track`))
  (bind _pushers (`self.pushers`))
  (bind _cartmover (`self.cartMover`))
  (bind _returnvalue (`KismetMathLibrary.Conv_IntToDouble` _pushers))
  (bind _returnvalue_2 (>= (`self.pushers`) 1))
  (bind _trackspline (`/Game/CustomMaps/UGC1662809422/BluePrints/PL/Track_Node.TrackSpline` (`self.Track`)))
  (bind _end_game_track (`/Game/CustomMaps/UGC1662809422/BluePrints/PL/Track_Node.End Game Track` _track))
  (bind _returnvalue_3 (`SplineComponent.GetSplineLength` _trackspline))
  (bind _returnvalue_4 (`KismetMathLibrary.Lerp` 0.0 _returnvalue_3 (`self.Alpha`)))
  (bind _returnvalue_5 (* (/ 50.0 (- _returnvalue_3 _returnvalue)) (`self.Default Speed Scale`)))
  (if (not (`/Game/CustomMaps/UGC1662809422/Pavlov_GravelWars.MatchEnded` (`self.GameLaws`)))
    (bind _playerstatus (`PavlovProxyStatics.GetPavlovPlayerStatusByPawn` (`GameplayStatics.GetPlayerCharacter` OtherBodyIndex)))
    (if (== (`.TeamId` (break `PavlovPlayerStatus` _playerstatus)) 0)
      (`/Engine/EditorBlueprintResources/ActorMacros.Switch Has Authority` :!label _label
        (:`Authority`
          (`self.MoveCartMulticast` :!label _label_2))
        (:`Remote`
          (`self.MoveCartServer`)))
      (else
        (bind (_direction _alpha) (`Timeline|cartMover` :!via `Stop` :!label _label_3)
          (:`Update`
            (if (>= _alpha (`/Game/CustomMaps/UGC1662809422/BluePrints/PL/Track_Node.When To Announce` (`self.Track`)))
              (if (`/Game/CustomMaps/UGC1662809422/BluePrints/PL/Track_Node.UseCapturePoint?` _track)
                (if (not (`self.alerted`)) :!label _label_4
                  (`/Game/CustomMaps/UGC1662809422/Pavlov_GravelWars.PayloadAlert` (`self.GameLaws`) _end_game_track)
                  (set `self.alerted` true))
                (elif _end_game_track
                  (goto _label_4)
                  (else
                    _))))
            (set `self.pushers` 0)
            (set `self.stop_push` false)
            (for _array_element (`PrimitiveComponent.GetOverlappingActors` (`self.PlayerSensor`) null)
              (bind _aspawn (cast `Pawn` _array_element))
              (bind _playerstatus_2 (`PavlovProxyStatics.GetPavlovPlayerStatusByPawn` _aspawn))
              (bind _returnvalue_6 (`Pavlov_Library.GetPlayerProxy` _aspawn))
              (if (`KismetSystemLibrary.IsValid` _returnvalue_6)
                (bind _playervitality (`Pavlov_PlayerProxy.GetPlayerVitality` _returnvalue_6))
                (if (not (`.bDead` (break `PlayerVitality` _playervitality)))
                  (bind _returnvalue_7 (`Pavlov_PlayerInfo.GetTeam` (`Pavlov_Library.GetPlayerInfo` (`.PlayerState` (break `PavlovPlayerStatus` _playerstatus_2)))))
                  (set `self.stop_push` (!= _returnvalue_7 (`self.Cart Team`)))
                  (set `self.pushers` (+ (`self.pushers`) 1)))))
            (if (>= _pushers 3)
              (`TimelineComponent.SetPlayRate` _cartmover (* _returnvalue_5 3.0))
              (elif (`self.Test The Cart`)
                (`TimelineComponent.SetPlayRate` _cartmover _returnvalue_5)
                (else
                  (`TimelineComponent.SetPlayRate` _cartmover (* _returnvalue _returnvalue_5)))))
            (if (`self.IsReversing?`)
              (if _returnvalue_2
                (set `self.reverse_check` false)
                (set `self.IsReversing?` false)
                (goto _label_3)
                (else
                  (bind _output_get (set `self.Alpha` _alpha :!label _label_5))
                  (set `self.CartStartOffset` _output_get)
                  (`self.K2_SetActorLocationAndRotation` (`SplineComponent.GetLocationAtDistanceAlongSpline` _trackspline _returnvalue_4 "World") (`SplineComponent.GetRotationAtDistanceAlongSpline` _trackspline _returnvalue_4 "World") :!label _label_6)))
              (elif (and _returnvalue_2 (not (`self.stop_push`)))
                (set `self.reverse_check` false :!label _label_7)
                (goto _label_5)
                (elif (`self.Test The Cart`)
                  (goto _label_7)
                  (else
                    (set `self.reverse_check` true)
                    (`|ExecutionSequence`
                      (:`then_0`
                        (goto _label_3 :!via `Stop`))
                      (:`then_1`
                        (if (`/Game/CustomMaps/UGC1662809422/BluePrints/PL/Track_Node.Hill Track` (`self.Track`))
                          (if _returnvalue_2 :!label _label_8
                            (set `self.IsReversing?` false)
                            (goto _label_3)
                            (else
                              (set `self.IsReversing?` true)
                              (goto _label_3 :!via `Reverse`)))
                          (else
                            (`KismetSystemLibrary.K2_SetTimerDelegate` (delegate `rollback_event`) 30.0))))))))))
          (:`Finished`
            (`|ExecutionSequence`
              (:`then_0`
                (if (== 0.0 _alpha)
                  _
                  (elif (not (`/Game/CustomMaps/UGC1662809422/Pavlov_GravelWars.MatchEnded` (`self.GameLaws`)))
                    (`/Engine/EditorBlueprintResources/ActorMacros.Switch Has Authority`
                      (:`Authority`
                        (`self.NextTrack` :!label _label_9))
                      (:`Remote`
                        (`self.NextTrackServer`))))))
              (:`then_1`
                (if (not _end_game_track)
                  (goto _label_3 :!via `SetNewTime`))))))))))

(event `self.ReceiveBeginPlay`
  (if (`self.ActiveCart`)
    (goto _label)))

(event `MoveCartServer`
  (goto _label_2))

(event `NextTrack`
  (bind _gamelaws (`self.GameLaws`))
  (bind _track (`self.Track`))
  (bind _next_track (`/Game/CustomMaps/UGC1662809422/BluePrints/PL/Track_Node.Next Track` _track))
  (if (`/Game/CustomMaps/UGC1662809422/BluePrints/PL/Track_Node.UseCapturePoint?` _track)
    (set `self.alerted` false)
    (`/Game/CustomMaps/UGC1662809422/BluePrints/PL/track_midcap_Blueprint.Capture` (`/Game/CustomMaps/UGC1662809422/BluePrints/PL/Track_Node.CapturePoint` _track)))
  (if (`/Game/CustomMaps/UGC1662809422/BluePrints/PL/Track_Node.End Game Track` _track)
    (`/Game/CustomMaps/UGC1662809422/Pavlov_GravelWars.EndRoundTF2` _gamelaws 0)
    (set `/Game/CustomMaps/UGC1662809422/Pavlov_GravelWars.RoundStatusCheck` 2 _gamelaws)
    (set `/Game/CustomMaps/UGC1662809422/Pavlov_GravelWars.PL_start_timer` 10 _gamelaws)
    (goto _label_3 :!via `Stop`)
    (else
      (set `self.CartStartOffset` 0.0)
      (`TimelineComponent.SetNewTime` (`self.cartMover`) 0.0)
      (if (`KismetSystemLibrary.IsValid` _next_track)
        (set `self.Track` _next_track)
        (`self.MoveCartMulticast`)
        (bind _output_get (set `self.Alpha` 0.0))
        (set `self.CartStartOffset` _output_get)
        (goto _label_6)))))

(event `NextTrackServer`
  (goto _label_9))

(event `MoveCartMulticast`
  (set `self.IsReversing?` false)
  (`TimelineComponent.SetNewTime` (`self.cartMover`) (`self.CartStartOffset`))
  (if (`self.CartSpawning?`)
    (set `self.CartSpawning?` false)
    (`|ExecutionSequence`
      (:`then_0`
        (goto _label_6))
      (:`then_1`
        (if (`/Game/CustomMaps/UGC1662809422/BluePrints/PL/Track_Node.Hill Track` (`self.Track`))
          (goto _label_3 :!via `Reverse`))))
    (else
      (goto _label_3))))

(event `rollback_event`
  (goto _label_8))

(fn `UserConstructionScript`)