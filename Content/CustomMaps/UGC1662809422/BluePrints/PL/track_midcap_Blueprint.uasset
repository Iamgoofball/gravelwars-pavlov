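; Mid-track capture point for a Payload mode map, with a beam and hologram that constantly rotate.
; On begin play it derives whether Red captures it from the assigned team's ID.
; Capture hides the default red visuals, shows the capturing team's, then updates GameLogic's payload stage, announces added time and extends the end timer.
; Server and multicast event pairs replicate the changes, while ResetVisuals restores the red look.
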(event `self.ReceiveTick`
  (params (DeltaSeconds :type "Float (single-precision)"))
  (`SceneComponent.K2_AddLocalRotation` (`self.Scene`) (struct :`Yaw` 0.4) false false))

(event `UnhideRedCapServer`
  (bind _game_logic (`self.Game Logic`))
  (`self.UnhideRedCapMulticast` :!label _label)
  (set `/Game/CustomMaps/UGC1662809422/Pavlov_GravelWars.Payload Stage` (`self.Spawns To Set`) _game_logic :!label _label_2)
  (if (`self.RedToCap?`)
    (`/Game/CustomMaps/UGC1662809422/Pavlov_GravelWars.PlayTimeAdded` _game_logic 1)
    (else
      (`/Game/CustomMaps/UGC1662809422/Pavlov_GravelWars.PlayTimeAdded` _game_logic 0)))
  (set `/Game/CustomMaps/UGC1662809422/Pavlov_GravelWars.PL_end_timer` (+ (`/Game/CustomMaps/UGC1662809422/Pavlov_GravelWars.PL_end_timer` _game_logic) 240) _game_logic))

(event `self.ReceiveBeginPlay`
  (`/Engine/EditorBlueprintResources/ActorMacros.Switch Has Authority`
    (:`Authority`
      (`self.SetIsRedCap?Multicast` :!label _label_3))
    (:`Remote`
      (`self.SetIsRedCap?Server`))))

(event `Capture`
  (`/Engine/EditorBlueprintResources/ActorMacros.Switch Has Authority`
    (:`Authority`
      (`self.HideDefaultCapMulticast` :!label _label_4)
      (if (`self.RedToCap?`)
        (`/Engine/EditorBlueprintResources/ActorMacros.Switch Has Authority`
          (:`Authority`
            (goto _label))
          (:`Remote`
            (`self.UnhideRedCapServer`)
            (goto _label_2)))
        (else
          (`/Engine/EditorBlueprintResources/ActorMacros.Switch Has Authority`
            (:`Authority`
              (`self.UnhideBluCapMulticast` :!label _label_5)
              (goto _label_2))
            (:`Remote`
              (`self.UnhideBluCapServer`)
              (goto _label_2))))))
    (:`Remote`
      (`self.HideDefaultCapServer`))))

(event `SetIsRedCap?Multicast`
  (if (not (== (`.TeamID` (break `GenericTeamId` (`self.TeamToCaptureIt`))) 0))
    (set `self.RedToCap?` true)))

(event `SetIsRedCap?Server`
  (goto _label_3))

(event `HideDefaultCapServer`
  (goto _label_4))

(event `UnhideBluCapServer`
  (goto _label_5))

(event `HideDefaultCapMulticast`
  (`SceneComponent.SetVisibility` (`self.CapPointBeam_Red`) false false)
  (`SceneComponent.SetVisibility` (`self.CapPointHologram_Red`) false false))

(event `UnhideRedCapMulticast`
  (`SceneComponent.SetVisibility` (`self.CapPointBeam_Red`) true false)
  (`SceneComponent.SetVisibility` (`self.CapPointHologram_Red`) true false))

(event `UnhideBluCapMulticast`
  (`SceneComponent.SetVisibility` (`self.CapPointBeam_Blu`) true false)
  (`SceneComponent.SetVisibility` (`self.CapPointHologram_Blu`) true false))

(event `ResetVisuals`
  (`SceneComponent.SetVisibility` (`self.CapPointBeam_Blu`) false false)
  (`SceneComponent.SetVisibility` (`self.CapPointHologram_Blu`) false false)
  (`SceneComponent.SetVisibility` (`self.CapPointBeam_Red`) true false)
  (`SceneComponent.SetVisibility` (`self.CapPointHologram_Red`) true false)
  (`SceneComponent.SetVisibility` (`self.CapPointBeam`) false false)
  (`SceneComponent.SetVisibility` (`self.CapPointHologram`) false false))

(fn `UserConstructionScript`)